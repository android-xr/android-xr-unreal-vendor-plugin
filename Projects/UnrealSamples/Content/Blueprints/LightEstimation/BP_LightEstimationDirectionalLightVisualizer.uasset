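; Visualizer actor that displays an estimated directional light on a sphere in XR.
; BeginPlay creates a dynamic material instance on the sphere, and UpdateVisualizer feeds the light's direction and color into its parameters.
; While ShouldMoveVisualizer is set, Tick interpolates the actor toward a fixed offset from the XRPawn's MenuTarget.
; EnableVisualizer passes Enabled straight to SetActorHiddenInGame, so true hides the actor.
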(event EventBeginPlay
  (bind _returnvalue (Rendering|Material|CreateDynamicMaterialInstance (Variables|Default|GetSphere) 0 "/Game/Materials/LightEstimation/M_LightEstimationDirectionalLight.M_LightEstimationDirectionalLight" "None" :!class /Script/Engine.PrimitiveComponent))
  (Variables|Default|SetDynamicMaterialInstance _returnvalue))

(event Collision|EventActorBeginOverlap
  (params (OtherActor :type Actor%20Object%20Reference)))

(event EventTick
  (params (DeltaSeconds :type Float%20%28single-precision%29))
  (if (Variables|Default|GetShould%20Move%20Visualizer)
    (bind _position (CallFunction|GetFollowPosition))
    (Transformation|SetActorLocation (Math|Interpolation|VInterpTo (Transformation|GetActorLocation) _position 0.0 0.0) false false)))

(fn ConstructionScript)

(fn UpdateVisualizer
  (params (DirectionalData :type Android%20XR%20Directional%20Light%20Data%20Structure%20%28by%20ref%29))
  (bind (_state _color _direction) (Utilities|Struct|BreakAndroidXRDirectionalLightData DirectionalData))
  (bind _dynamicmaterialinstance (Variables|Default|GetDynamicMaterialInstance))
  (Rendering|Material|SetVectorParameterValue _dynamicmaterialinstance "Direction" (Math|Conversions|ToLinearColor(Vector) _direction) :!class /Script/Engine.MaterialInstanceDynamic)
  (Rendering|Material|SetVectorParameterValue _dynamicmaterialinstance "Color" _color :!class /Script/Engine.MaterialInstanceDynamic))

(fn GetFollowPosition
  (bind _asxrpawn (Utilities|Casting|CastToXRPawn (Game|Player|GetPlayerPawn 0)))
  (return (+ (Transformation|GetWorldLocation (Variables|/Game/XRPawn.XRPawn_C|GetMenuTarget _asxrpawn)) "10.000000,0.000000,0.000000")))

(fn ShouldMoveVisualizer
  (params (ShouldMoveVisualizer :type Boolean))
  (Variables|Default|SetShould%20Move%20Visualizer ShouldMoveVisualizer))

(fn EnableVisualizer
  (params (Enabled :type Boolean))
  (Rendering|SetActorHiddenInGame Enabled))