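; Actor representing an Android XR spatial anchor, with a cube outline whose color shows persistence state.
; Wraps the AndroidXRSpatialAnchors component to create or adopt an anchor, persist, unpersist or load it, and destroy it with the actor.
; BeginPlay binds persistence callbacks that recolor a dynamic material: green for persisted, white for unpersisted, red for failure.
; Initialize's tint for already-persisted entities targets parameter "None" instead of "Color".
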(event Custom|OnAnchorPersisted
  (Rendering|Material|SetVectorParameterValue (Variables|Default|GetMaterialnstance) "Color" "(R=0.085728,G=1.000000,B=0.149460,A=1.000000)" :!class /Script/Engine.MaterialInstanceDynamic))

(event Custom|OnAnchorUnpersisted
  (Rendering|Material|SetVectorParameterValue (Variables|Default|GetMaterialnstance) "Color" "(R=1.000000,G=0.990133,B=1.000000,A=1.000000)" :!class /Script/Engine.MaterialInstanceDynamic))

(event Custom|OnAnchorPersistFailed
  (params (FailureReason :type ESpatialAnchorPeristenceResult%20Enum :default "Success"))
  (Rendering|Material|SetVectorParameterValue (Variables|Default|GetMaterialnstance) "Color" "(R=1.000000,G=0.051352,B=0.006189,A=1.000000)" :!class /Script/Engine.MaterialInstanceDynamic))

(event Custom|OnAnchorUnpersistFailed
  (params (FailureReason :type ESpatialAnchorPeristenceResult%20Enum :default "Success"))
  (Rendering|Material|SetVectorParameterValue (Variables|Default|GetMaterialnstance) "Color" "(R=1.000000,G=0.051352,B=0.006189,A=1.000000)" :!class /Script/Engine.MaterialInstanceDynamic))

(event EventBeginPlay
  (bind _androidxrspatialanchors (Variables|Default|GetAndroidXRSpatialAnchors))
  (Utilities|FlowControl|Sequence
    (:then_0
      (EventDispatchers|AssignOnAnchorPersisted _androidxrspatialanchors (delegate Custom|OnAnchorPersisted))
      (EventDispatchers|AssignOnAnchorUnpersisted _androidxrspatialanchors (delegate Custom|OnAnchorUnpersisted))
      (EventDispatchers|AssignOnAnchorPersistFailed _androidxrspatialanchors (delegate Custom|OnAnchorPersistFailed))
      (EventDispatchers|AssignOnAnchorUnpersistFailed _androidxrspatialanchors (delegate Custom|OnAnchorUnpersistFailed))
      (bind _returnvalue (Rendering|Material|CreateDynamicMaterialInstance "/Game/Materials/M_SpatialAnchorOutline.M_SpatialAnchorOutline" "None" "None" :!class /Script/Engine.KismetMaterialLibrary))
      (bind _output_get (Variables|Default|SetMaterialnstance _returnvalue))
      (Rendering|Material|SetMaterial (Variables|Default|GetCube) 0 _output_get))))

(event Collision|EventActorBeginOverlap
  (params (OtherActor :type Actor%20Object%20Reference)))

(event EventTick
  (params (DeltaSeconds :type Float%20%28single-precision%29)))

(event EventDestroyed
  (Class|AndroidXRSpatialAnchorsComponent|DestroyAnchor (Variables|Default|GetAndroidXRSpatialAnchors)))

(fn ConstructionScript)

(fn PersistAnchor
  (if (not (Variables|Default|GetPersistedAnchor))
    (Class|AndroidXRSpatialAnchorsComponent|PersistAnchor (Variables|Default|GetAndroidXRSpatialAnchors))))

(fn UnpersistAnchor
  (Class|AndroidXRSpatialAnchorsComponent|UnpersistAnchor (Variables|Default|GetAndroidXRSpatialAnchors)))

(fn LoadPersistedAnchor
  (params (Anchor :type Android%20XR%20Spatial%20Anchor%20Entity%20Object%20Reference))
  (Class|AndroidXRSpatialAnchorsComponent|Initialize (Variables|Default|GetAndroidXRSpatialAnchors) Anchor)
  (Rendering|Material|SetVectorParameterValue (Variables|Default|GetMaterialnstance) "Color" "(R=0.340815,G=1.000000,B=0.276996,A=1.000000)" :!class /Script/Engine.MaterialInstanceDynamic))

(fn Initialize
  (params (Entity :type Android%20XR%20Spatial%20Anchor%20Entity%20Object%20Reference))
  (Utilities|IsValid Entity
    (:Is%20Valid
      (Class|AndroidXRSpatialAnchorsComponent|Initialize (Variables|Default|GetAndroidXRSpatialAnchors) Entity)
      (if (Variables|/Script/AndroidXRSpatialAnchors.AndroidXRSpatialAnchorEntity|GetbIsPersisted Entity)
        (Rendering|Material|SetVectorParameterValue (Variables|Default|GetMaterialnstance) "None" "(R=0.137559,G=1.000000,B=0.053318,A=1.000000)" :!class /Script/Engine.MaterialInstanceDynamic)))
    (:Is%20Not%20Valid
      (Class|AndroidXRSpatialAnchorsComponent|CreateAnchor (Variables|Default|GetAndroidXRSpatialAnchors)))))