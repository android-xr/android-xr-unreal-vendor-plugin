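; Manager actor for Android XR spatial marker tracking that shows each detected marker as a BP_SpatialMarkerActor.
; Marker notifier events spawn and initialize an actor for an added marker, or destroy it on removal, using MarkerTable to map markers to actors.
; Configure, StartTracking and StopTracking forward to the marker tracking subsystem.
; Destroying the manager destroys all spawned marker actors and clears the table.
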(event OnMarkerAdded(AndroidXRSpatialMarkersNotifier)
  (params (Marker :type Android%20XR%20Spatial%20Marker%20Entity%20Object%20Reference))
  (bind _returnvalue (Game|SpawnActorfromClass "/Game/Blueprints/SpatialEntities/MarkerTracking/BP_SpatialMarkerActor.BP_SpatialMarkerActor_C" (Math|Transform|MakeTransform "0, 0, 0") "Undefined" "MultiplyWithRoot" 0 0))
  (Default|Initialize _returnvalue Marker)
  (Utilities|Map|Add (Variables|Default|GetMarkerTable) Marker _returnvalue))

(event OnMarkerRemoved(AndroidXRSpatialMarkersNotifier)
  (params (Marker :type Android%20XR%20Spatial%20Marker%20Entity%20Object%20Reference))
  (bind _markertable (Variables|Default|GetMarkerTable))
  (bind (_value _returnvalue) (Utilities|Map|Find _markertable Marker))
  (if _returnvalue
    (Actor|DestroyActor _value)
    (Utilities|Map|Remove _markertable Marker)))

(event EventBeginPlay)

(event Collision|EventActorBeginOverlap
  (params (OtherActor :type Actor%20Object%20Reference)))

(event EventDestroyed
  (bind _markertable (Variables|Default|GetMarkerTable))
  (bind _valuepin (Utilities|Map|ForEachLoop(Map) _markertable)
    (:then
      (Actor|DestroyActor _valuepin))
    (:CompletedPin
      (Utilities|Map|Clear _markertable))))

(fn ConstructionScript)

(fn Configure
  (params (Config :type Spatial%20Marker%20Tracking%20Config%20Structure%20%28by%20ref%29))
  (Class|AndroidXRSpatialMarkerTrackingSubsystem|ConfigureMarkerTracking (|AndroidXRSpatialMarkerTrackingSubsystem) Config))

(fn StartTracking
  (Class|AndroidXRTrackingSubsystem|StartTracking (|AndroidXRSpatialMarkerTrackingSubsystem)))

(fn StopTracking
  (Class|AndroidXRTrackingSubsystem|StopTracking (|AndroidXRSpatialMarkerTrackingSubsystem)))