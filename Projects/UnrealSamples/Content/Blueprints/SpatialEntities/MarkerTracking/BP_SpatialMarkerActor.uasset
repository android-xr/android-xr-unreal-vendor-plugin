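; BP_SpatialMarkerActor visualizes a tracked spatial marker entity with a plane, a coordinate-system gizmo and a text label.
; Initialize stores the marker entity, and Tick reapplies its data every frame while it stays valid.
; ApplyData aligns the plane and gizmo to the marker transform, dividing marker size by mesh bounds to scale the plane.
; The unrotated label shows the marker type with its string data, or its ID when none exists.
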(event EventBeginPlay)

(event Collision|EventActorBeginOverlap
  (params (OtherActor :type Actor%20Object%20Reference)))

(event EventTick
  (params (DeltaSeconds :type Float%20%28single-precision%29))
  (bind _marker_entity (Variables|Default|GetMarker%20Entity))
  (Utilities|IsValid _marker_entity
    (:Is%20Valid
      (CallFunction|ApplyData _marker_entity))))

(fn ConstructionScript)

(fn Initialize
  (params (MarkerEntity :type Android%20XR%20Spatial%20Marker%20Entity%20Object%20Reference%20%28by%20ref%29))
  (CallFunction|ApplyData MarkerEntity)
  (Variables|Default|SetMarker%20Entity MarkerEntity))

(fn ApplyData
  (params (MarkerInfo :type Android%20XR%20Spatial%20Marker%20Entity%20Object%20Reference%20%28by%20ref%29))
  (bind _plane (Variables|Default|GetPlane))
  (bind _markertransform (Variables|/Script/AndroidXRSpatialMarkerTracking.AndroidXRSpatialMarkerEntity|GetMarkerTransform MarkerInfo))
  (bind _textrender (Variables|Default|GetTextRender))
  (bind _markertype (Variables|/Script/AndroidXRSpatialMarkerTracking.AndroidXRSpatialMarkerEntity|GetMarkerType MarkerInfo))
  (bind _markertransform_2 (Variables|/Script/AndroidXRSpatialMarkerTracking.AndroidXRSpatialMarkerEntity|GetMarkerTransform MarkerInfo))
  (bind _markerscale (Variables|/Script/AndroidXRSpatialMarkerTracking.AndroidXRSpatialMarkerEntity|GetMarkerScale MarkerInfo))
  (bind (_location _rotation) (Math|Transform|BreakTransform _markertransform_2))
  (bind (_x _y) (Math|Vector2D|BreakVector2D _markerscale))
  (bind (_location_2 _rotation_2) (Math|Transform|BreakTransform _markertransform))
  (bind _returnvalue (Utilities|String|EnumtoString _markertype))
  (bind _staticmesh (Variables|/Script/Engine.StaticMeshComponent|GetStaticMesh _plane))
  (bind _returnvalue_2 (StaticMesh|GetBounds _staticmesh))
  (bind _boxextent (Math|BoxSphereBounds|BreakBoxSphereBounds _returnvalue_2))
  (bind (_x_2 _y_2 _z) (Math|Vector|BreakVector _boxextent))
  (Utilities|FlowControl|Sequence
    (:then_0
      (Transformation|SetWorldTransform (Variables|Default|GetPlane) (Math|Transform|MakeTransform _location _rotation (Math|Vector|MakeVector 0.01 (/ _x _y_2) (/ _y _z))) false false))
    (:then_1
      (Transformation|SetWorldTransform (Variables|Default|GetCoordinateSystem) (Math|Transform|MakeTransform _location_2 _rotation_2 "0.450000,0.450000,0.450000") false false))
    (:then_2
      (if (Variables|/Script/AndroidXRSpatialMarkerTracking.AndroidXRSpatialMarkerEntity|GetbHasStringData MarkerInfo)
        (Rendering|Components|TextRender|SetText _textrender (Utilities|Text|FormatText "{Type} {Data}" _returnvalue (Variables|/Script/AndroidXRSpatialMarkerTracking.AndroidXRSpatialMarkerEntity|GetMarkerStringData MarkerInfo)))
        (else
          (Rendering|Components|TextRender|SetText _textrender (Utilities|Text|FormatText "{Type}: {Id}" _returnvalue (Variables|/Script/AndroidXRSpatialMarkerTracking.AndroidXRSpatialMarkerEntity|GetMarkerId MarkerInfo))))))
    (:then_3
      (Transformation|SetWorldTransform _textrender (Math|Transform|MakeTransform (.Location (Math|Transform|BreakTransform (Variables|/Script/AndroidXRSpatialMarkerTracking.AndroidXRSpatialMarkerEntity|GetMarkerTransform MarkerInfo))) "0, 0, 0" "0.250000,0.250000,0.250000") false false))))