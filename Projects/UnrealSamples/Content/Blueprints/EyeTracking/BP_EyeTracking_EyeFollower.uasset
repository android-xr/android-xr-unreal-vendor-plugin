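; BP_EyeTracking_EyeFollower is an eye actor for Android XR eye tracking, with a colored component for each eye.
; BeginPlay tints both eyes and starts tracking through the AndroidXREyeTrackingSubsystem, and Destroyed stops it.
; Helper functions switch fine tracking mode and return the RightEyeTracking component's eye state, flagged valid when it holds at least two eyes.
; The graphs contain no per-frame movement logic.
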(event EventBeginPlay
  (Rendering|Material|SetColorParameterValueonMaterials (Variables|Default|GetRightEye) "Color" (Math|Conversions|ToLinearColor(Color) (Variables|Default|GetRightEyeColor)))
  (Rendering|Material|SetColorParameterValueonMaterials (Variables|Default|GetLeftEye) "Color" (Math|Conversions|ToLinearColor(Color) (Variables|Default|GetLeftEyeColor)))
  (Class|AndroidXRTrackingSubsystem|StartTracking (|AndroidXREyeTrackingSubsystem)))

(event Collision|EventActorBeginOverlap
  (params (OtherActor :type Actor%20Object%20Reference)))

(event EventTick
  (params (DeltaSeconds :type Float%20%28single-precision%29)))

(event EventDestroyed
  (Class|AndroidXRTrackingSubsystem|StopTracking (|AndroidXREyeTrackingSubsystem)))

(fn ConstructionScript)

(fn SetEyeTrackingMode
  (params (IsFineMode :type Boolean))
  (Class|AndroidXREyeTrackingSubsystem|SetEyeTrackingMode (|AndroidXREyeTrackingSubsystem) IsFineMode))

(fn GetEyeTrackingData
  (bind _righteyetracking (Variables|Default|GetRightEyeTracking))
  (bind _eyesstate (Variables|/Script/AndroidXREyeTracking.AndroidXREyeTrackingComponent|GetEyesState _righteyetracking))
  (return _eyesstate (>= (Utilities|Array|Length (.Eyes (Utilities|Struct|BreakAndroidXREyes _eyesstate))) 2)))