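; Actor that visualizes an Android XR anchor with a colored cube and a text label, and destroys its space when destroyed.
; A dynamic material shows selection, location and persistence state, while the text shows persisted ID, state and trackable binding.
; Async calls persist or unpersist the anchor through the game state's AnchorPersistence.
; Looping timers support polling persist state and retrying space location, which moves the actor once located.
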(event EventBeginPlay
  (|CallParentFunction)
  (bind _returnvalue (Rendering|Material|CreateDynamicMaterialInstance (Variables|Default|GetCube) 0 (Rendering|Material|GetMaterial (Variables|Default|GetCube) 0) "None" :!class /Script/Engine.PrimitiveComponent))
  (bind _output_get (Variables|Default|SetMaterialInstance _returnvalue))
  (Rendering|Material|SetMaterial (Variables|Default|GetCube) 0 _output_get)
  (Variables|Default|SetGameStateRaycast (.AsXRGame%20State%20Trackables%20Core (Utilities|Casting|CastToXRGameStateTrackablesCore (Game|GetGameState)))))

(event Collision|EventActorBeginOverlap
  (params (OtherActor :type Actor%20Object%20Reference))
  (|CallParentFunction OtherActor) ; This node is disabled and will not be called.\nDrag off pins to build functionality.
)

(event EventTick
  (params (DeltaSeconds :type Float%20%28single-precision%29))
  (|CallParentFunction DeltaSeconds) ; This node is disabled and will not be called.\nDrag off pins to build functionality.
)

(event EventDestroyed
  ;[0.15 0.15 0.15 0.5] Calling xrDestroySpace on persisted spaces seems to break things
  (Class|AndroidXRBlueprintFunctionLibrary|DestroySpace (.Space (Utilities|Struct|BreakAndroidXRAnchor (Variables|Default|GetAnchor)))))

(event Custom|OnPersistAnchor
  (params (AnchorPersistence :type Android%20XR%20Anchor%20Persistence%20Structure%20%28by%20ref%29) (AnchorSpace :type Android%20XR%20Space%20Structure%20%28by%20ref%29))
  (bind _anchor (Variables|Default|GetAnchor))
  (bind (_anchorspace _persistedid) (|PersistAnchorAsync AnchorPersistence AnchorSpace)
    (:OnAnchorPersisted
      (Utilities|Struct|SetmembersinAndroidXRAnchor _anchor _anchorspace _persistedid (.Transform (Utilities|Struct|BreakAndroidXRAnchor _anchor))))))

(event Custom|OnUnpersistAnchor
  (params (AnchorPersistence :type Android%20XR%20Anchor%20Persistence%20Structure%20%28by%20ref%29) (PersistedId :type Guid%20Structure%20%28by%20ref%29))
  (bind _anchor (Variables|Default|GetAnchor))
  (bind (_space _persistedid _transform) (Utilities|Struct|BreakAndroidXRAnchor _anchor))
  (|UnpersistAnchorAsync AnchorPersistence PersistedId
    (:OnAnchorUnpersisted
      (Utilities|Struct|SetmembersinAndroidXRAnchor _anchor _space "00000000000000000000000000000000" _transform)
      (CallFunction|UpdateText (Utilities|Enum|LiteralenumEAndroidXRAnchorPersistState "PersistNotRequested")))))

(fn ConstructionScript
  (bind _trackable (Variables|Default|GetTrackable))
  (bind _returnvalue (Class|AndroidXRTrackablesCoreBlueprintFunctionLibrary|IsValidTrackable _trackable))
  (|CallParentFunction)
  (Transformation|SetRelativeLocationAndRotation (Variables|Default|GetTextRender) (select _returnvalue "10.000000,8.000000,0.000000" "0.000000,8.000000,10.000000") (select _returnvalue "90.000000,90.000000,0.000000" "0.000000,180.000000,0.000000") false false))

(fn Init
  (params (Anchor :type Android%20XR%20Anchor%20Structure) (State :type EAndroidXRAnchorPersistState%20Enum :default "PersistNotRequested") (IsLocated :type Boolean))
  (Variables|Default|SetIsLocated IsLocated)
  (Variables|Default|SetAnchor Anchor)
  (CallFunction|UpdateText State)
  (CallFunction|UpdateColor))

(fn SetSelected
  (params (Selected :type Boolean))
  (Variables|Default|SetSelected Selected)
  (CallFunction|UpdateColor))

(fn UpdateColor
  (Rendering|Material|SetVectorParameterValue (Variables|Default|GetMaterialInstance) "Color" (Math|Color|SelectColor "(R=1.000000,G=1.000000,B=0.000000,A=1.000000)" (Math|Color|SelectColor (Math|Color|SelectColor "(R=0.000000,G=1.000000,B=0.000000,A=1.000000)" "(R=1.000000,G=1.000000,B=1.000000,A=1.000000)" (CallFunction|IsPersisted)) "(R=1.000000,G=0.000000,B=0.000000,A=1.000000)" (Variables|Default|GetIsLocated)) (Variables|Default|GetSelected)) :!class /Script/Engine.MaterialInstanceDynamic))

(fn IsPersisted
  (return (Guid|IsValidGuid (.PersistedID (Utilities|Struct|BreakAndroidXRAnchor (Variables|Default|GetAnchor))))))

(fn BeginPersist
  (CallFunction|OnPersistAnchor (Variables|/Game/XRGameStateTrackablesCore.XRGameStateTrackablesCore_C|GetAnchorPersistence (Variables|Default|GetGameStateRaycast)) (.Space (Utilities|Struct|BreakAndroidXRAnchor (Variables|Default|GetAnchor))))
  (Variables|Default|SetIsPollingPersistStatus true)
  (bind _returnvalue (Utilities|Time|SetTimerbyEvent (EventDispatchers|CreateEvent :!event PollPersistState) 0.25 true))
  (Variables|Default|SetPersistPollTimer _returnvalue))

(fn PollPersistState
  (bind _anchor (Variables|Default|GetAnchor))
  (bind _persistedid (Utilities|Struct|BreakAndroidXRAnchor _anchor))
  (if (Guid|IsValidGuid _persistedid)
    (bind (_persiststate _returnvalue) (Class|AndroidXRAnchorPersistenceBlueprintFunctionLibrary|GetAnchorPersistState (Variables|/Game/XRGameStateTrackablesCore.XRGameStateTrackablesCore_C|GetAnchorPersistence (Variables|Default|GetGameStateRaycast)) _persistedid))
    (if _returnvalue
      (Utilities|FlowControl|Sequence
        (:then_0
          (switch Utilities|FlowControl|Switch|SwitchonEAndroidXRAnchorPersistState _persiststate
            (:PersistNotRequested
              _)
            (:Persisted
              _))
          (Utilities|Time|ClearandInvalidateTimerbyHandle (Variables|Default|GetPersistPollTimer))
          (Variables|Default|SetIsPollingPersistStatus false))
        (:then_1
          (CallFunction|UpdateText _persiststate))))))

(fn UpdateText
  (params (State :type Byte :default 0))
  (Rendering|Components|TextRender|SetText (Variables|Default|GetTextRender) (Utilities|Text|FormatText "{ID}
{State}
{Trackable}" (Guid|ToString(Guid) (.PersistedID (Utilities|Struct|BreakAndroidXRAnchor (Variables|Default|GetAnchor)))) (|GenerictoText State) (Utilities|String|SelectString "Bound to Trackable" "" (Class|AndroidXRTrackablesCoreBlueprintFunctionLibrary|IsValidTrackable (Variables|Default|GetTrackable))))))

(fn Unpersist
  (CallFunction|OnUnpersistAnchor (Variables|/Game/XRGameStateTrackablesCore.XRGameStateTrackablesCore_C|GetAnchorPersistence (Variables|Default|GetGameStateRaycast)) (.PersistedID (Utilities|Struct|BreakAndroidXRAnchor (Variables|Default|GetAnchor)))))

(fn LocateSpace
  (bind (_transform _returnvalue) (Class|AndroidXRBlueprintFunctionLibrary|LocateSpace (.Space (Utilities|Struct|BreakAndroidXRAnchor (Variables|Default|GetAnchor)))))
  (if _returnvalue
    (Variables|Default|SetIsLocated true)
    (Transformation|SetActorTransform _transform)
    (Utilities|Time|ClearandInvalidateTimerbyHandle (Variables|Default|GetUpdateLocationTimer))
    (CallFunction|UpdateColor)))

(fn BeginLocatingSpace
  (bind _returnvalue (Utilities|Time|SetTimerbyEvent (EventDispatchers|CreateEvent :!event LocateSpace) 0.25 true))
  (Variables|Default|SetUpdateLocationTimer _returnvalue))